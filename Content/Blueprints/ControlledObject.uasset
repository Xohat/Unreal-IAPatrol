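; An actor the player drags around the level with the mouse, keeping its current height.
; Clicking the Body component opens a Gate on Tick and releasing closes it; while open, the actor moves to the X/Y of a complex Camera-channel trace under the cursor.
; BeginPlay caches MyPlayerController, which supplies that trace and switches the cursor to a hand while hovering over Body.
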(event `self.ReceiveBeginPlay`
  ;[1 1 1] Guarda el material inicial del objeto y se obtiene el player Controller
  (bind _asmy_player_controller (cast `/Game/Blueprints/MyPlayerController` (`GameplayStatics.GetPlayerController` 0)))
  (set `self.Player Controller` _asmy_player_controller))

(event `self.ReceiveTick`
  (params (DeltaSeconds :type "Float (single-precision)"))
  ;[1 1 1] Getión de la mecánica de pulsaciones, materiales y seguimiento del objeto
  (`/Engine/EditorBlueprintResources/StandardMacros.Gate` true :!label _label
    (:`Exit`
      ;[1 1 1] Gestión de la posición del cursor y la posición del objeto
      (`self.K2_SetActorLocation` (`KismetMathLibrary.MakeVector` (.x (`.Location` (`GameplayStatics.BreakHitResult` (`PlayerController.GetHitResultUnderCursorByChannel` (`self.Player Controller`) "TraceTypeQuery2" true)))) (.y (`.Location` (`GameplayStatics.BreakHitResult` (`PlayerController.GetHitResultUnderCursorByChannel` (`self.Player Controller`) "TraceTypeQuery2" true)))) (.z (`self.K2_GetActorLocation`)))))))

(event `self.Body.OnClicked`
  (params (TouchedComponent :type "PrimitiveComponent Object Reference") (ButtonPressed :type "Key Structure"))
  ;[1 1 1] Getión de la mecánica de pulsaciones, materiales y seguimiento del objeto
  (goto _label :!via `Open`))

(event `self.Body.OnReleased`
  (params (TouchedComponent :type "PrimitiveComponent Object Reference") (ButtonReleased :type "Key Structure"))
  ;[1 1 1] Getión de la mecánica de pulsaciones, materiales y seguimiento del objeto
  (goto _label :!via `Close`))

(event `self.Body.OnBeginCursorOver`
  (params (TouchedComponent :type "PrimitiveComponent Object Reference"))
  ;[1 1 1] Gestión de la apariencia cursor
  (set `PlayerController.CurrentMouseCursor` "Hand" (`self.Player Controller`)))

(event `self.Body.OnEndCursorOver`
  (params (TouchedComponent :type "PrimitiveComponent Object Reference"))
  ;[1 1 1] Gestión de la apariencia cursor
  (set `PlayerController.CurrentMouseCursor` "Default" (`self.Player Controller`)))

(fn `UserConstructionScript`)